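; Test actor that moves its Cube component back and forth along the local Y axis.
; The construction script stores the cube's starting relative location.
; Each tick adds Speed times delta time to Y without sweeping, then flips the sign of Speed once the cube is more than a fixed distance from that start.
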(event `self.ReceiveTick`
  (params (DeltaSeconds :type "Float (single-precision)"))
  (bind _cube (`self.Cube`))
  (bind (_startpos_x _startpos_y) (`KismetMathLibrary.BreakVector` (`self.StartPos`)))
  (bind (_relativelocation_x _relativelocation_y _relativelocation_z) (`KismetMathLibrary.BreakVector` (`SceneComponent.RelativeLocation` _cube)))
  ;[1 1 1] p=p0+vt
  ;;[1 1 1] vt
  (`SceneComponent.K2_SetRelativeLocation` _cube (`KismetMathLibrary.MakeVector` _relativelocation_x (+ (* DeltaSeconds (`self.Speed`)) _relativelocation_y) _relativelocation_z) false false)
  (if (> (`KismetMathLibrary.Abs` (- _relativelocation_y _startpos_y)) 500.0)
    (set `self.Speed` (* (`self.Speed`) -1.0))))

(fn `UserConstructionScript`
  (set `self.StartPos` (`SceneComponent.RelativeLocation` (`self.Cube`))))