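; BP_KYJ is a movement test Blueprint that slides its Cube component back and forth along the relative Y axis.
; Each Tick moves the cube by Speed scaled by delta time, in the direction given by the IsMoveRight flag.
; When the cube passes a fixed limit on either side of the origin, the flag flips to reverse travel, with no sweep collision checks.
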(event `self.ReceiveTick`
  (params (DeltaSeconds :type "Float (single-precision)"))
  (bind _cube (`self.Cube`))
  (bind (_relativelocation_x _relativelocation_y) (`KismetMathLibrary.BreakVector` (`SceneComponent.RelativeLocation` (`self.Cube`))))
  (bind (_relativelocation_x_2 _relativelocation_y_2) (`KismetMathLibrary.BreakVector` (`SceneComponent.RelativeLocation` (`self.Cube`))))
  ;[1 1 1] Adjust Speed
  (set `self.Delta Location` (`KismetMathLibrary.MakeVector` 0.0 (* DeltaSeconds (`self.Speed`))))
  (if (`self.isMoveRight`)
    (`SceneComponent.K2_AddRelativeLocation` _cube (`self.Delta Location`) false false) ; 위치 조정
    (if (> _relativelocation_y_2 1000.0)
      (set `self.isMoveRight` false))
    (else
      (`SceneComponent.K2_AddRelativeLocation` _cube (* (`self.Delta Location`) (0.0 -1.0 0.0)) false false) ; 위치 조정
      (if (< _relativelocation_y -1000.0)
        (set `self.isMoveRight` true)))))

(fn `UserConstructionScript`)