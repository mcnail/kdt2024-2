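; Prototype password dial actor that builds a numbered ring around a Cylinder.
; The construction script divides 360 degrees by Count, then accumulates yaw to place a centered number label and a sphere collision at each step.
; Labels and spheres attach to the Cylinder, and the spheres are stored in CollArr.
; The Checker component's overlap event only prints a placeholder "Hello", with no password logic yet.
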(event `self.Checker.OnComponentBeginOverlap`
  (params (OverlappedComponent :type "PrimitiveComponent Object Reference") (OtherActor :type "Actor Object Reference") (OtherComp :type "PrimitiveComponent Object Reference") (OtherBodyIndex :type Integer) (bFromSweep :type Boolean) (SweepResult :type "HitResult Structure (by ref)"))
  (if (!= OtherComp null)
    (`KismetSystemLibrary.PrintString` "Hello")))

(fn `UserConstructionScript`
  (bind _count (`self.count`))
  (bind (_arrrot_roll _arrrot_pitch _arrrot_yaw) (`KismetMathLibrary.BreakRotator` (`self.arrRot`)))
  (bind _arrrot (`self.arrRot`))
  (`KismetArrayLibrary.Array_Clear` (`self.collArr`)) ; 배열을 비운다
  (set `self.angle` (/ 360.0 (`KismetMathLibrary.Conv_IntToDouble` _count)))
  ;[1 1 1] for(int i = First Index ; i <= last Index ; i++)
  ;;[1 1 1] 반복한다 = for loop
  (for _index (range _count)
    ;[1 1 1] 반복한다
    ;;[1 1 1] 텍스트 렌더러 컴포넌트 를 배치한다
    (bind _returnvalue (`AddComponent|NODE_AddTextRenderComponent-0` :`RelativeTransform` (`KismetMathLibrary.MakeTransform` (* (`KismetMathLibrary.GetForwardVector` _arrrot) 51.0) _arrrot)))
    (`TextRenderComponent.K2_SetText` _returnvalue (`KismetTextLibrary.Conv_IntToText` _index))
    (`TextRenderComponent.SetHorizontalAlignment` _returnvalue "EHTA_Center")
    (`TextRenderComponent.SetVerticalAlignment` _returnvalue "EVRTA_TextCenter")
    (`TextRenderComponent.SetTextRenderColor` _returnvalue (make `Color` 0 0 1))
    (`SceneComponent.K2_AttachToComponent` _returnvalue (`self.Cylinder`) "None" "KeepRelative" "KeepRelative" "KeepWorld" true) ; Target : Text // Parent : Cylinder
    ;;[1 1 1] 스피어 컬리전을 추가
    (bind _returnvalue_2 (`AddComponent|NODE_AddSphereComponent-0` :`RelativeTransform` (`KismetMathLibrary.MakeTransform` (* (`KismetMathLibrary.GetForwardVector` (`self.arrRot`)) 57.0))))
    (`KismetArrayLibrary.Array_Add` (`self.collArr`) _returnvalue_2) ; Item 추가
    (`SceneComponent.K2_AttachToComponent` _returnvalue_2 (`self.Cylinder`) "None" "KeepRelative" "KeepRelative" "KeepRelative" true) ; Target : Text // Parent : Cylinder
    ;;[1 1 1] Angle 만큼 회전을 누적 한다
    (set `self.arrRot` (`KismetMathLibrary.MakeRotator` _arrrot_roll _arrrot_pitch (+ _arrrot_yaw (`self.angle`))))))