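; BP_Follow is a prototype pickup actor that trails the player character once its PickedUP event fires.
; While picked up, Tick steps it toward the player whenever it falls behind a set distance, until Sphere1 hits something other than the player.
; BeginPlay creates a dynamic dissolve material on the Sphere, with parameters set through DynaMatChange.
; Orbit, attach and timed dissolve-then-destroy logic is left disconnected, and Box overlap only prints test text.
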(event `self.ReceiveBeginPlay`
  ;[1 1 1] I will Change to Parameter in Material
  (bind _returnvalue (`PrimitiveComponent.CreateDynamicMaterialInstance` (`self.Sphere`) 0 "/Game/Proto/Materials/MI_dissolve.MI_dissolve" "None"))
  (set `self.dissolveMat` _returnvalue)
  (`self.DynaMatChange` 1.0 0.05 10.0))

(event `self.Sphere1.OnComponentHit`
  (params (HitComponent :type "PrimitiveComponent Object Reference") (OtherActor :type "Actor Object Reference") (OtherComp :type "PrimitiveComponent Object Reference") (NormalImpulse :type "Vector Structure") (Hit :type "HitResult Structure (by ref)"))
  (bind _asbp_third_person_character (cast `/Game/ThirdPerson/Blueprints/BP_ThirdPersonCharacter` (`GameplayStatics.GetPlayerCharacter` 0)))
  (if (not (== OtherActor _asbp_third_person_character))
    ;[1 1 1] 히트 된 대상(other)가 플레이어라면
    (set `self.is Player` false)))

(event `FollowUp`
  ;[1 1 1] 나(픽업오브젝트, self)의 위치를 (플레이어 앞으로) 업데이트  해라!
  (`self.K2_SetActorLocation` (+ (`self.K2_GetActorLocation` (`GameplayStatics.GetPlayerCharacter` 0)) (* (`self.roundVector`) 110.0)) true))

(event `self.ReceiveTick`
  (params (DeltaSeconds :type "Float (single-precision)"))
  (bind _returnvalue (`self.K2_GetActorLocation`))
  (bind _returnvalue_2 (`self.K2_GetActorLocation` (`GameplayStatics.GetPlayerCharacter` 0)))
  (if (and (>= (`KismetMathLibrary.Vector_Distance` _returnvalue_2 _returnvalue) 150.0) (`self.is Player`))
    (`self.K2_SetActorLocation` (+ (`self.K2_GetActorLocation`) (* (`KismetMathLibrary.Normal` (- _returnvalue_2 _returnvalue)) 50.0)))))

(event `/Game/Proto/BP/BP_pickup_Itfc.PickedUP`
  (set `self.is Player` true))

(event `self.Box.OnComponentBeginOverlap`
  (params (OverlappedComponent :type "PrimitiveComponent Object Reference") (OtherActor :type "Actor Object Reference") (OtherComp :type "PrimitiveComponent Object Reference") (OtherBodyIndex :type Integer) (bFromSweep :type Boolean) (SweepResult :type "HitResult Structure (by ref)"))
  (`KismetSystemLibrary.PrintString` "BOX test"))

(fn `UserConstructionScript`)