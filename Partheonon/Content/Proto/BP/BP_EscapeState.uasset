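; BP_EscapeState runs the time-limit timer for what its name suggests is an escape prototype.
; BeginPlay creates the UI_Timer widget and adds it to the viewport.
; Tick accumulates elapsed time and, while it is below LimitTime, pushes the progress ratio and a formatted minute-and-second text into the widget.
; Reaching the limit only stops these updates, as the debug prints, including the time-up message, are unconnected.
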(event `self.ReceiveBeginPlay`
  (bind _returnvalue (`|CreateWidget` "/Game/Proto/UI/UI_Timer.UI_Timer_C"))
  (bind _output_get (set `self.uiTimerRef` _returnvalue))
  (`UserWidget.AddToViewport` _output_get 0))

(event `self.ReceiveTick`
  (params (DeltaSeconds :type "Float (single-precision)"))
  ;[1 1 1] Timer
  (bind _output_get (set `self.curTime` (+ DeltaSeconds (`self.curTime`))))
  (if (not (>= _output_get (`self.limitTime`)))
    (`self.ProgUpdate`)
    (`self.TimeTextUpdate`)))

(event `ProgUpdate`
  ;[1 1 1] 프로그래스바 업데이트 : 부분 / 전체 = 비율
  (set `/Game/Proto/UI/UI_Timer.timeRatio` (/ (`self.curTime`) (`self.limitTime`)) (`self.uiTimerRef`)))

(event `TimeTextUpdate`
  (bind _curtime (`self.curTime`))
  ;[1 1 1] UI time text update
  (set `/Game/Proto/UI/UI_Timer.timeText` (`|FormatText` "{min} : {sec}" (`KismetTextLibrary.Conv_DoubleToText` (/ _curtime 60.0) "ToZero" false true 2 2 0 0) (`KismetTextLibrary.Conv_DoubleToText` (mod _curtime 60.0) "ToZero" false true 2 2 0 0)) (`self.uiTimerRef`)))

(fn `UserConstructionScript`)