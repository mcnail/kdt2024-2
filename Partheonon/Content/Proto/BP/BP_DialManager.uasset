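; BP_DialManager is a combination-dial puzzle manager, apparently for an escape game, that checks child BP_Dial actors against a password.
; The construction script sizes the answer array to the password and spawns one child-actor dial per entry, stacked downward.
; GetDialsCurNum records each dial's match, then PasswordChecker prints the result.
; On full success it calls AnswerAllTrue, locks as solved and notifies BP_EscapeState through CheckDialManager.
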(event `GetDialsCurNum`
  (bind _answerarr (`self.answerArr`))
  ;[1 1 1] Child BP_Dial 의 curNum를 가지고 온다
  (if (not (`self.isSolved`))
    (for (_ _array_index) (`self.passwordArr`)
      ;;[1 1 1] curNum와 passwordArr를 비교한다
      (bind _asbp_dial (cast `/Game/Proto/Password/BP_Dial` (`ChildActorComponent.ChildActor` (`|GetArrayItem` (`self.dialArr`) _array_index))))
      (if (== (`/Game/Proto/Password/BP_Dial.curNum` _asbp_dial) (`|GetArrayItem` (`self.passwordArr`) _array_index))
        ;;;[1 1 1] 비교한 결과를 answerArr에 저장
        (`KismetArrayLibrary.Array_Set` _answerarr _array_index true)
        (else
          (`KismetArrayLibrary.Array_Set` _answerarr _array_index))))
    (`self.PasswordChecker`)))

(event `PasswordChecker`
  ;[1 1 1] 정답을 확인한다 == answerArr
  (if (`KismetArrayLibrary.Array_Contains` (`self.answerArr`))
    (`KismetSystemLibrary.PrintString` "더 분발하세요")
    (else
      (`KismetSystemLibrary.PrintString` "정답입니다")
      (`self.AnswerAllTrue`)
      (set `self.isSolved` true)
      (bind _asbp_escape_state (cast `/Game/Proto/BP/BP_EscapeState` (`GameplayStatics.GetGameState`)))
      (`/Game/Proto/BP/BP_EscapeState.CheckDialManager` _asbp_escape_state))))

(fn `UserConstructionScript`
  (bind _answerarr (`self.answerArr`))
  (bind (_dialloc_x _dialloc_y _dialloc_z) (`KismetMathLibrary.BreakVector` (`self.dialLoc`)))
  (bind _returnvalue (`KismetArrayLibrary.Array_Length` (`self.passwordArr`)))
  ;[1 1 1] 배열초기화
  (`KismetArrayLibrary.Array_Clear` _answerarr)
  (`KismetArrayLibrary.Array_Resize` _answerarr _returnvalue)
  ;[1 1 1] 차일드 액터 추가
  (for _ (range _returnvalue)
    (bind _returnvalue_2 (`AddComponent|NODE_AddChildActorComponent-0` :`RelativeTransform` (`KismetMathLibrary.MakeTransform` (`self.dialLoc`))))
    (`KismetArrayLibrary.Array_Add` (`self.dialArr`) _returnvalue_2)
    (set `self.dialLoc` (`KismetMathLibrary.MakeVector` _dialloc_x _dialloc_y (+ _dialloc_z -40.0)))))