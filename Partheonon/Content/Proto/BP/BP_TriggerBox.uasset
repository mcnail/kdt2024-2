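; BP_TriggerBox is a trigger actor that slides a gate mesh vertically when the player's third-person character enters or leaves its overlap area.
; Entering plays the GateSliding timeline and leaving reverses it.
; Each timeline update adds MoveZ times Speed to the gate's current relative Z, so movement accumulates rather than interpolating between fixed positions.
; Speed flips sign whenever the timeline finishes, switching the travel direction.
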(event `self.ReceiveBeginPlay`)

(event `self.ReceiveActorBeginOverlap`
  (params (OtherActor :type "Actor Object Reference"))
  (bind _sm_gate (`self.SM_Gate`))
  (bind (_relativelocation_x _relativelocation_y _relativelocation_z) (`KismetMathLibrary.BreakVector` (`SceneComponent.RelativeLocation` _sm_gate)))
  ;[1 1 1] 플레이어가 트리거 영역에 들어오면
  (bind _asbp_third_person_character (cast `/Game/ThirdPerson/Blueprints/BP_ThirdPersonCharacter` OtherActor))
  (`/Engine/EditorBlueprintResources/StandardMacros.IsValid` _asbp_third_person_character
    (:`Is Valid`
      (if (== _asbp_third_person_character (`GameplayStatics.GetPlayerPawn` 0))
        ;[1 1 1] 문을 위에서 아래로 슬라이딩 되라(이동 해라)
        (bind (_direction _movez) (`Timeline|GateSliding` :!label _label)
          (:`Update`
            (`SceneComponent.K2_SetRelativeLocation` _sm_gate (`KismetMathLibrary.MakeVector` _relativelocation_x _relativelocation_y (+ _relativelocation_z (* _movez (`self.speed`)))) false false))
          (:`Finished`
            ;;[1 1 1] 움직이는 방향을 업데이트(반대로)
            (set `self.speed` (* (`self.speed`) -1.0))))))))

(event `self.ReceiveActorEndOverlap`
  (params (OtherActor :type "Actor Object Reference"))
  ;[1 1 1] 플레이어가 컬리전 영역에 벗어나면
  (bind _asbp_third_person_character (cast `/Game/ThirdPerson/Blueprints/BP_ThirdPersonCharacter` OtherActor))
  (`/Engine/EditorBlueprintResources/StandardMacros.IsValid` _asbp_third_person_character
    (:`Is Valid`
      (if (== _asbp_third_person_character (`GameplayStatics.GetPlayerPawn` 0))
        (goto _label :!via `Reverse`)))))

(event `self.ReceiveTick`
  (params (DeltaSeconds :type "Float (single-precision)")))

(event `self.Box.OnComponentEndOverlap`
  (params (OverlappedComponent :type "PrimitiveComponent Object Reference") (OtherActor :type "Actor Object Reference") (OtherComp :type "PrimitiveComponent Object Reference") (OtherBodyIndex :type Integer)))

(fn `UserConstructionScript`)